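; BP_Resource is an actor representing a harvestable resource with a finite number of units.
; Its Harvest function takes a desired amount, subtracts up to that many from UnitsLeft and returns the amount actually collected.
; The actor destroys itself once depleted, and its event graph and construction script hold no active logic.
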(fn `Harvest`
  (params (DesiredAmount :type Integer))
  (returns (CollectdAmount :type Integer))
  (locals (Collected :type Integer))
  ;[1 1 1] Determine Collected Amount
  (bind _output_get (set `local.Collected` (`KismetMathLibrary.Min` DesiredAmount (`self.Units Left`))))
  (bind _output_get_2 (set `self.Units Left` (- (`self.Units Left`) _output_get)))
  ;[1 1 1] Check has Depleted
  (if (<= _output_get_2 0)
    (`self.K2_DestroyActor`))
  (return (`local.Collected`)))

(fn `UserConstructionScript`)