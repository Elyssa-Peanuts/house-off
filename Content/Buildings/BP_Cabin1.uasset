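; BP_Cabin1 is a cabin building that earns coins for the game state once constructed.
; It extends a parent building's construction logic, adding a slight rotation to the Cabin component on BeginPlay.
; When construction ends, a looping timer calls PayTaxes, which adds BP_Coin to BP_GameState at a regular interval.
; SetColourByState only calls CanBePlaced, with no colour logic of its own.
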(event `self.ReceiveBeginPlay`
  (`parent.ReceiveBeginPlay`)
  (`SceneComponent.K2_AddLocalRotation` (`self.Cabin`) (struct :`Yaw` 3.0) false false))

(fn `EndConstructing`
  (`parent.EndConstructing`)
  (`KismetSystemLibrary.K2_SetTimer` null "PayTaxes" 10.0 true))

(fn `PayTaxes`
  (bind _asbp_game_state (cast `/Game/Blueprints/BP_GameState` (`GameplayStatics.GetGameState`)))
  (`/Game/Blueprints/BP_GameState.AddResourceAmount` _asbp_game_state "/Game/Resources/BP_Coin.BP_Coin_C" 10))

(fn `Set Colour By State`
  (`self.CanBePlaced`))

(fn `UserConstructionScript`
  (`parent.UserConstructionScript`))