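; BP_Mason1 is a mason building that extends a parent building class and shows a stone icon on its resource widget.
; BeginPlay sets that icon after the parent logic runs.
; SetColourByState swaps the mesh to green or red forge materials while floating, based on placement validity, and to the normal forge material when ready.
; Processing start and end toggle a fire particle system around the parent logic, while DoProcessing is empty.
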(event `self.ReceiveBeginPlay`
  ;[1 1 1] Set Icon
  (`parent.ReceiveBeginPlay`)
  (bind _aswbp_resource_icon (cast `/Game/Buildings/WBP_ResourceIcon` (`WidgetComponent.GetUserWidgetObject` (`self.Resource_Icon`))))
  (set `/Game/Buildings/WBP_ResourceIcon.ResourceIcon` (make `SlateBrush` "Image" "NoTile" "NoMirror" (make `DeprecateSlateVector2D` 512.0 512.0) (struct) (struct :`SpecifiedColor` (struct :`R` 1.0 :`G` 1.0 :`B` 1.0 :`A` 1.0) :`ColorUseRule` "UseColor_Specified") (struct :`CornerRadii` (struct) :`Color` (struct :`SpecifiedColor` (struct) :`ColorUseRule` "UseColor_Specified") :`RoundingType` "HalfHeightRadius") "/Game/UI/Stone.Stone") _aswbp_resource_icon))

(fn `DoProcessing`)

(fn `EndProcessing`
  (params (CollectedAmount :type Integer))
  (`parent.EndProcessing` CollectedAmount)
  (`ActorComponent.Deactivate` (`self.PS_Fire`)))

(fn `Set Colour By State`
  (bind _result (`self.CanBePlaced`))
  (`PrimitiveComponent.SetMaterial` (`self.Mason`) 0 (select `/Game/Buildings/E_State` (`self.State`) :`NewEnumerator0` (select `bool` _result :`false` "/Game/Materials/M_ForgeRed.M_ForgeRed" :`true` "/Game/Materials/M_ForgeGreen.M_ForgeGreen" :!type "MaterialInterface Object Reference") :`NewEnumerator1` "/Game/Materials/M_Forge.M_Forge")))

(fn `StartProcessing`
  (`parent.StartProcessing`)
  (`ActorComponent.Activate` (`self.PS_Fire`) false))

(fn `UserConstructionScript`
  (`parent.UserConstructionScript`))