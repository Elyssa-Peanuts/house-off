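; Base building actor that the player places, then builds over a short timer before it becomes ready.
; While floating, its bounds turn green or red depending on whether the game state can cover its costs and no other buildings overlap it, tracked through overlap events.
; Placing it plays a sound and shows a spinning construction indicator until the timer finishes, then the bounds turn white.
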(event `self.ReceiveActorBeginOverlap`
  (params (OtherActor :type "Actor Object Reference"))
  (bind _asbp_building (cast `/Game/Buildings/BP_Building` OtherActor))
  (`BlueprintSetLibrary.Set_Add` (`self.Overlapped Buildings`) _asbp_building))

(event `self.ReceiveActorEndOverlap`
  (params (OtherActor :type "Actor Object Reference"))
  (bind _asbp_building (cast `/Game/Buildings/BP_Building` OtherActor))
  (`BlueprintSetLibrary.Set_Remove` (`self.Overlapped Buildings`) _asbp_building))

(event `self.ReceiveTick`
  (params (DeltaSeconds :type "Float (single-precision)"))
  (`self.Set Colour By State`)
  (switch `/Game/Buildings/E_State` (`self.State`)
    (:`NewEnumerator4`
      (`SceneComponent.K2_AddWorldRotation` (`self.Constructing`) (struct :`Yaw` 1.0) false false))))

(fn `CanBePlaced`
  (returns (Result :type Boolean))
  ;[1 1 1] Can costs be covered?
  (bind _asbp_game_state (cast `/Game/Blueprints/BP_GameState` (`GameplayStatics.GetGameState`)))
  (bind _result (`/Game/Blueprints/BP_GameState.AreCostsCovered` _asbp_game_state (`self.Costs`)))
  (return (and _result (== (`BlueprintSetLibrary.Set_Length` (`self.Overlapped Buildings`)) 0))))

(fn `EndConstructing`
  (`SceneComponent.SetHiddenInGame` (`self.Constructing`) true false)
  (set `self.State` "NewEnumerator1"))

(fn `Place Building`
  (set `self.State` "NewEnumerator4")
  (`KismetSystemLibrary.K2_SetTimer` null "EndConstructing" 5.0)
  (`SceneComponent.SetHiddenInGame` (`self.Constructing`) false false)
  (`GameplayStatics.PlaySound2D` "/Game/UI/epic-object-placing-105779.epic-object-placing-105779" 1.0 1.0 0.0 null null))

(fn `Set Colour By State`
  (bind _result (`self.CanBePlaced`))
  (`PrimitiveComponent.SetMaterial` (`self.Bounds`) 0 (select `/Game/Buildings/E_State` (`self.State`) :`NewEnumerator0` (select `bool` _result :`false` "/Game/Materials/M_Red.M_Red" :`true` "/Game/Materials/M_Green.M_Green" :!type "MaterialInterface Object Reference") :`NewEnumerator1` "/Game/Materials/M_White.M_White")))

(fn `UserConstructionScript`)