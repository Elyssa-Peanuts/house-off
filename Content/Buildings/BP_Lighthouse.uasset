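; Lighthouse building Blueprint that overrides placement-colour and processing functions, likely from a shared building parent class.
; Set Colour By State calls CanBePlaced and sets the skeletal mesh's first material slot.
; Each DoProcessing call rotates the skeletal mesh by a fixed local step, while EndProcessing runs the parent logic and plays a 2D collect sound.
; BeginPlay, overlap and Tick are disabled stubs.
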(fn `DoProcessing`
  (`SceneComponent.K2_AddLocalRotation` (`self.SkeletalMesh`) (struct :`Yaw` 10.0) false false))

(fn `EndProcessing`
  (params (CollectedAmount :type Integer))
  (`parent.EndProcessing` CollectedAmount)
  (`GameplayStatics.PlaySound2D` "/Game/UI/collect-5930.collect-5930" 1.0 1.0 0.0 null null))

(fn `Set Colour By State`
  (`self.CanBePlaced`)
  (`PrimitiveComponent.SetMaterial` (`self.SkeletalMesh`) 0 null))

(fn `UserConstructionScript`
  (`parent.UserConstructionScript`))