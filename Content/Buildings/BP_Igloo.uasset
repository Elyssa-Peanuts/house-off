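; Igloo building, a placeable child of a parent building class, that shows a drinks icon on its resource widget.
; SetColourByState tints the mesh green or red by placement validity while floating and restores its normal material when ready.
; Processing overrides turn the fire particle effect on at start and off at end, nudging the igloo's rotation on start and on each DoProcessing call.
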(event `self.ReceiveBeginPlay`
  ;[1 1 1] Set Icon
  (`parent.ReceiveBeginPlay`)
  (bind _aswbp_resource_icon (cast `/Game/Buildings/WBP_ResourceIcon` (`WidgetComponent.GetUserWidgetObject` (`self.Resource_Icon`))))
  (set `/Game/Buildings/WBP_ResourceIcon.ResourceIcon` (make `SlateBrush` "Image" "NoTile" "NoMirror" (make `DeprecateSlateVector2D` 512.0 512.0) (struct) (struct :`SpecifiedColor` (struct :`R` 1.0 :`G` 1.0 :`B` 1.0 :`A` 1.0) :`ColorUseRule` "UseColor_Specified") (struct :`CornerRadii` (struct) :`Color` (struct :`SpecifiedColor` (struct) :`ColorUseRule` "UseColor_Specified") :`RoundingType` "HalfHeightRadius") "/Game/UI/drinksIcon.drinksIcon") _aswbp_resource_icon))

(fn `DoProcessing`
  (`SceneComponent.K2_AddLocalRotation` (`self.Igloo`) (struct :`Yaw` 2.0) false false))

(fn `EndProcessing`
  (params (CollectedAmount :type Integer))
  (`parent.EndProcessing` CollectedAmount)
  (`ActorComponent.Deactivate` (`self.PS_Fire`)))

(fn `Set Colour By State`
  (bind _result (`self.CanBePlaced`))
  (`PrimitiveComponent.SetMaterial` (`self.Igloo`) 0 (select `/Game/Buildings/E_State` (`self.State`) :`NewEnumerator0` (select `bool` _result :`false` "/Game/Elyssa/Materials/Red.Red" :`true` "/Game/Elyssa/Materials/Green.Green" :!type "MaterialInterface Object Reference") :`NewEnumerator1` "/Game/Elyssa/Materials/Material_001.Material_001")))

(fn `StartProcessing`
  (`parent.StartProcessing`)
  (`ActorComponent.Activate` (`self.PS_Fire`) false)
  (`SceneComponent.K2_AddLocalRotation` (`self.Igloo`) (struct :`Yaw` 2.0) false false))

(fn `UserConstructionScript`
  (`parent.UserConstructionScript`))