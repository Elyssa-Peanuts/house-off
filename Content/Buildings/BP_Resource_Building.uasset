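; Base resource building that produces a resource and credits it to the game state.
; StartProcessing sets the processing state, during which Tick calls DoProcessing, an empty hook in this class.
; EndProcessing returns to ready, adds the collected amount, and briefly shows an animated widget icon, hidden again by timer.
; When construction ends, it starts the loop on its child-actor worker.
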(event `self.ReceiveTick`
  (params (DeltaSeconds :type "Float (single-precision)"))
  (`parent.ReceiveTick` DeltaSeconds)
  (switch `/Game/Buildings/E_State` (`self.State`)
    (:`NewEnumerator2`
      (`self.DoProcessing`))))

(fn `DoProcessing`)

(fn `EndConstructing`
  (`parent.EndConstructing`)
  (bind _asbp_worker (cast `/Game/Characters/BP_Worker` (`ChildActorComponent.ChildActor` (`self.BP_Worker`))))
  (`/Game/Characters/BP_Worker.StartLoop` _asbp_worker))

(fn `EndProcessing`
  (params (CollectedAmount :type Integer))
  (set `self.State` "NewEnumerator1")
  (bind _asbp_game_state (cast `/Game/Blueprints/BP_GameState` (`GameplayStatics.GetGameState`)))
  (`/Game/Blueprints/BP_GameState.AddResourceAmount` _asbp_game_state (`self.ResourceClass`) CollectedAmount)
  (`SceneComponent.SetHiddenInGame` (`self.Resource_Icon`) false false)
  (`KismetSystemLibrary.K2_SetTimer` null "Hide_Resource_Icon" 5.0)
  (bind _aswbp_resource_icon (cast `/Game/Buildings/WBP_ResourceIcon` (`WidgetComponent.GetUserWidgetObject` (`self.Resource_Icon`))))
  (`/Game/Buildings/WBP_ResourceIcon.Animate` _aswbp_resource_icon))

(fn `Hide_Resource_Icon`
  (`SceneComponent.SetHiddenInGame` (`self.Resource_Icon`) true false))

(fn `StartProcessing`
  (set `self.State` "NewEnumerator2"))

(fn `UserConstructionScript`
  (`parent.UserConstructionScript`))