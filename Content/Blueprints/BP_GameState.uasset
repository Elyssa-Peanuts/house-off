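; Game state that keeps the player's resource stockpile and handles building costs.
; On BeginPlay it creates the top bar widget and seeds starting tent, bar and coin amounts.
; A class-to-amount map holds the totals, with every change routed through SetResourceAmount to update the bar.
; AreCostsCovered compares a cost map against the stock, and PayforBuilding deducts costs by adding negated amounts.
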(event `self.ReceiveBeginPlay`
  (bind _returnvalue (`|CreateWidget` "/Game/UI/WBP_TopBar.WBP_TopBar_C"))
  (`UserWidget.AddToViewport` _returnvalue 0)
  (set `self.ResourceBar` _returnvalue)
  (`self.SetResourceAmount` "/Game/Resources/BP_Tent.BP_Tent_C" 30)
  (`self.SetResourceAmount` "/Game/Resources/BP_Bar.BP_Bar_C" 50)
  (`self.SetResourceAmount` "/Game/Resources/BP_Coin.BP_Coin_C" 10))

(fn `AddResourceAmount`
  (params (ResourceClass :type "/Game/Resources/BP_Resource Class Reference") (ResourceAmount :type Integer))
  (bind (_value _returnvalue) (`BlueprintMapLibrary.Map_Find` (`self.ResourceMap`) ResourceClass))
  (if _returnvalue
    (`self.SetResourceAmount` ResourceClass (+ ResourceAmount _value))
    (else
      (`self.SetResourceAmount` ResourceClass ResourceAmount))))

(fn `AreCostsCovered`
  (params (Costs :type "Map of /Game/Resources/BP_Resource Class Reference to Integer"))
  (returns (Result :type Boolean))
  (locals (TempResult :type Boolean :default true))
  (bind _keys (`BlueprintMapLibrary.Map_Keys` Costs))
  (for _array_element _keys
    ;[1 1 1] Check every resource
    (if (not (>= (`BlueprintMapLibrary.Map_Find` (`self.ResourceMap`) _array_element) (`BlueprintMapLibrary.Map_Find` Costs _array_element)))
      (set `local.TempResult` false)
      (break)))
  (return (`local.TempResult`)))

(fn `PayforBuilding`
  (params (Costs :type "Map of /Game/Resources/BP_Resource Class Reference to Integer"))
  (locals (TempResult :type Boolean :default true))
  (bind _keys (`BlueprintMapLibrary.Map_Keys` Costs))
  ;[1 1 1] Takes the Amount and Multiplies it by -1
  (for _array_element _keys
    (`self.AddResourceAmount` _array_element (* (`BlueprintMapLibrary.Map_Find` Costs _array_element) -1))))

(fn `SetResourceAmount`
  (params (ResourceClass :type "/Game/Resources/BP_Resource Class Reference") (ResourceAmount :type Integer))
  (`BlueprintMapLibrary.Map_Add` (`self.ResourceMap`) ResourceClass ResourceAmount)
  (`/Game/UI/WBP_TopBar.SetResourceAmount` (`self.ResourceBar`) ResourceClass ResourceAmount))

(fn `UserConstructionScript`)