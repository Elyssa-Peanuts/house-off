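; Camera pawn that shows the mouse cursor and provides pan, rotate and zoom controls.
; Each Tick polls Enhanced Input values, applying keyboard movement, strafe and yaw as frame-rate-scaled local offsets and rotations.
; Middle-mouse drag pans, otherwise right-mouse drag yaws, and only with neither held does zoom adjust spring arm length.
; Zoom is not delta-time scaled, and steps landing outside the arm length limits are skipped rather than clamped.
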(event `self.ReceiveBeginPlay`
  (set `PlayerController.bShowMouseCursor` true (`GameplayStatics.GetPlayerController` 0)))

(event `self.ReceiveTick`
  (params (DeltaSeconds :type "Float (single-precision)"))
  (bind (_returnvalue_x _returnvalue_y) (`KismetMathLibrary.BreakVector2D` (`|GetInputActionValue`)))
  (bind _maxcameraspeed (`self.MaxCameraSpeed`))
  (bind _springarm (`self.SpringArm`))
  (bind _returnvalue (+ (* (`|GetInputActionValue`) (`self.CameraZoomSpeed`)) (`SpringArmComponent.TargetArmLength` _springarm)))
  ;[1 1 1] Move Camera by K/B
  (`self.K2_AddActorLocalOffset` (* (`KismetMathLibrary.GetForwardVector` (struct)) (`|GetInputActionValue`) (`self.MaxCameraSpeed`) DeltaSeconds))
  ;[1 1 1] Strafe Camera by K/B
  (`self.K2_AddActorLocalOffset` (* (`KismetMathLibrary.GetRightVector` (struct)) (`|GetInputActionValue`) (`self.MaxCameraSpeed`) DeltaSeconds))
  ;[1 1 1] Rotate Camera by K/B
  (`self.K2_AddActorLocalRotation` (`KismetMathLibrary.MakeRotator` 0.0 0.0 (* (`|GetInputActionValue`) DeltaSeconds (`self.CameraRotationSpeed`))))
  ;[1 1 1] Move Camera by Mouse
  (if (`PlayerController.IsInputKeyDown` (`GameplayStatics.GetPlayerController` 0) "MiddleMouseButton")
    (`self.K2_AddActorLocalOffset` (+ (* (`KismetMathLibrary.GetForwardVector` (struct)) _maxcameraspeed _returnvalue_y DeltaSeconds) (* (`KismetMathLibrary.GetRightVector` (struct)) _returnvalue_x _maxcameraspeed DeltaSeconds)))
    (else
      ;[1 1 1] Rotate Camera by Mouse
      (if (`PlayerController.IsInputKeyDown` (`GameplayStatics.GetPlayerController` 0) "RightMouseButton")
        (`self.K2_AddActorLocalRotation` (`KismetMathLibrary.MakeRotator` 0.0 0.0 (* _returnvalue_x (`self.CameraRotationSpeed`) DeltaSeconds)))
        (else
          ;[1 1 1] Zoom Camera
          (if (and (<= _returnvalue (`self.MaxArmLength`)) (>= _returnvalue (`self.MinArmLength`)))
            (set `SpringArmComponent.TargetArmLength` _returnvalue _springarm)))))))

(fn `UserConstructionScript`)